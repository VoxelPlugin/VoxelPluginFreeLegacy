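; Bouncing sphere modifier that deforms voxel terrain where it hits a VoxelChunk with enough impact strength.
; On hit, it converts the hit point to voxel-local space and loops over a sphere of Radius around it.
; Each voxel value is increased in proportion to its magnitude (minimum one) and the impact strength.
; Changed voxels are queued, then applied in one update when the loop completes.
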(event OnComponentHit(StaticMeshComponent)
  (params (HitComponent :type Primitive%20Component%20Object%20Reference) (OtherActor :type Actor%20Object%20Reference) (OtherComp :type Primitive%20Component%20Object%20Reference) (NormalImpulse :type Vector :default "0, 0, 0") (Hit :type Hit%20Result%20Structure%20%28by%20ref%29))
  (if (>= (Utilities|GetImpactStrength) 0.1)
    (Utilities|IsValid OtherActor
      (:Is%20Valid
        (if (== (Utilities|GetClass OtherActor) "/Script/Voxel.VoxelChunk")
          (bind _asvoxel_world (Utilities|Casting|CastToVoxelWorld (Actor|GetAttachParentActor OtherActor)))
          (bind _pointposition (Utilities|SphereLoopInt (|AddUpVector (Class|VoxelWorld|GlobaltoLocal _asvoxel_world (.Location (Collision|BreakHitResult Hit)))) (Variables|Default|GetRadius) 1.0 1.0 1.0)
            (:Loop%20body
              (Class|VoxelWorld|SetValue _asvoxel_world _pointposition (+ (Class|VoxelWorld|GetValue _asvoxel_world _pointposition) (* (Math|Float|Max(Float) (Math|Float|Absolute(Float) (Class|VoxelWorld|GetValue _asvoxel_world _pointposition)) 1.0) (Utilities|GetImpactStrength))))
              (Class|VoxelWorld|QueueUpdate _asvoxel_world _pointposition))
            (:Completed
              (Class|VoxelWorld|ApplyQueuedUpdates _asvoxel_world false))))))))

(fn ConstructionScript)