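; Voxel world actor that periodically runs a water effect on its own voxel data.
; Tick skips its first frame, then accumulates delta time and calls ApplyWaterEffect on itself with a fixed radius and speed whenever the short update interval has elapsed.
; The timer resets to zero after each call, throttling the effect independently of frame rate.
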(event EventTick
  (params (DeltaSeconds :type Float%20%28single-precision%29))
  (if (Variables|Default|GetFirstTickSkipped)
    (bind _output_get (Variables|Default|SetTimeSinceUpdate (+ DeltaSeconds (Variables|Default|GetTimeSinceUpdate))))
    (if (> _output_get 0.05)
      (Class|VoxelTools|ApplyWaterEffect self "0, 0, 0" 1e+01 0.1)
      (Variables|Default|SetTimeSinceUpdate 0.0))
    (else
      (Variables|Default|SetFirstTickSkipped true))))

(fn ConstructionScript)