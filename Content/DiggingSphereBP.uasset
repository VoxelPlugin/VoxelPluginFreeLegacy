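; DiggingSphereBP is an actor that carves a sphere out of voxel terrain when its static mesh hits it.
; On hit, it checks the other actor's class, gets the parent VoxelWorld and converts the impact point to local voxel coordinates.
; A SphereLoopInt loop around that offset point removes voxels using Radius and Strength, queuing each update and applying them all once the loop completes.
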(event OnComponentHit(StaticMeshComponent)
  (params (HitComponent :type Primitive%20Component%20Object%20Reference) (OtherActor :type Actor%20Object%20Reference) (OtherComp :type Primitive%20Component%20Object%20Reference) (NormalImpulse :type Vector :default "0, 0, 0") (Hit :type Hit%20Result%20Structure%20%28by%20ref%29))
  (bind _radius (Variables|Default|GetRadius))
  (Utilities|IsValid OtherActor
    (:Is%20Valid
      (if (== (Utilities|GetClass OtherActor) 0)
        (bind _asvoxel_world (Utilities|Casting|CastToVoxelWorld (Actor|GetAttachParentActor OtherActor)))
        (bind _returnvalue (Class|VoxelWorld|GlobaltoLocal _asvoxel_world (.Location (Collision|BreakHitResult Hit))))
        (bind _pointposition (Utilities|SphereLoopInt (|AddUpVector_2 _returnvalue) _radius 1.0 1.0 (/ 1.0 _radius))
          (:Loop%20body
            (Class|VoxelWorld|Remove _asvoxel_world _pointposition (Variables|Default|GetStrength))
            (Class|VoxelWorld|QueueUpdate _asvoxel_world _pointposition))
          (:Completed
            (Class|VoxelWorld|ApplyQueuedUpdates _asvoxel_world false)))))))

(fn ConstructionScript)