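; VoxelSpline is a spline-based placeable item that registers data items along its path in a voxel world.
; On AddItemtoWorld, each pair of adjacent spline points becomes a segment in voxel-local coordinates, added to the world's PlaceableItemManager.
; Each segment carries a cached generator instance, mask, start, end and radius, with bounds padded by the scaled radius.
; Segments are straight between points, so curvature between them is not sampled.
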(event EventAddItemtoWorld
  (params (World :type Voxel%20World%20Object%20Reference))
  (bind _spline (Variables|Default|GetSpline))
  (bind _radius (Variables|Default|GetRadius))
  (for _index (range 0 (- (Spline|GetNumberOfSplinePoints (Variables|Default|GetSpline)) 2))
    (|AddDataItem (Variables|/Script/Voxel.VoxelWorld|GetPlaceableItemManager World) (Class|VoxelGeneratorCache|MakeGeneratorInstance (Class|VoxelWorld|GetGeneratorCache World) (Variables|Default|GetGenerator)) (Class|VoxelIntBoxLibrary|Extend (Class|VoxelIntBoxLibrary|MakeIntBoxfromPoints (Utilities|Array|MakeArray (Class|VoxelWorld|GlobaltoLocalFloat World (Spline|GetLocationatSplinePoint _spline _index "World")) (Class|VoxelWorld|GlobaltoLocalFloat World (Spline|GetLocationatSplinePoint _spline (+ _index 1) "World")))) (Math|Float|Ceil (* (Variables|Default|GetBounds%20Multiplier) _radius))) (Variables|Default|GetMask) (.X (Math|Vector|BreakVector (Class|VoxelWorld|GlobaltoLocalFloat World (Spline|GetLocationatSplinePoint _spline _index "World")))) (.Y (Math|Vector|BreakVector (Class|VoxelWorld|GlobaltoLocalFloat World (Spline|GetLocationatSplinePoint _spline _index "World")))) (.Z (Math|Vector|BreakVector (Class|VoxelWorld|GlobaltoLocalFloat World (Spline|GetLocationatSplinePoint _spline _index "World")))) (.X (Math|Vector|BreakVector (Class|VoxelWorld|GlobaltoLocalFloat World (Spline|GetLocationatSplinePoint _spline (+ _index 1) "World")))) (.Y (Math|Vector|BreakVector (Class|VoxelWorld|GlobaltoLocalFloat World (Spline|GetLocationatSplinePoint _spline (+ _index 1) "World")))) (.Z (Math|Vector|BreakVector (Class|VoxelWorld|GlobaltoLocalFloat World (Spline|GetLocationatSplinePoint _spline (+ _index 1) "World")))) _radius)))

(fn ConstructionScript)