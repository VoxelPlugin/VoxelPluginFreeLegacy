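; Blueprint function library for Voxel worlds that reports which surface materials lie at a given position.
; GetMultiIndexMaterialsAtPosition finds the closest non-empty voxel and decodes its multi-index material, sorted by strength.
; It resolves the four indices through the world's material collection and returns those materials with their strengths and wetness.
; When no voxel is found, it returns failure with zeroed values.
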(fn GetMultiIndexMaterialsatPosition
  (params (Voxel%20World :type Voxel%20World%20Object%20Reference) (Position :type Vector))
  (bind _materialcollection (Variables|/Script/Voxel.VoxelWorld|GetMaterialCollection Voxel%20World))
  (bind _result (Class|VoxelDataTools|FindClosestNonEmptyVoxel Voxel%20World Position))
  (if (.bsuccess _result)
    (return true (Class|VoxelMaterialCollectionBase|GetIndexMaterial _materialcollection (.Index0 (Class|VoxelBlueprintLibrary|GetMultiIndex (.material _result) true))) (.Strength0 (Class|VoxelBlueprintLibrary|GetMultiIndex (.material _result) true)) (Class|VoxelMaterialCollectionBase|GetIndexMaterial _materialcollection (.Index1 (Class|VoxelBlueprintLibrary|GetMultiIndex (.material _result) true))) (.Strength1 (Class|VoxelBlueprintLibrary|GetMultiIndex (.material _result) true)) (Class|VoxelMaterialCollectionBase|GetIndexMaterial _materialcollection (.Index2 (Class|VoxelBlueprintLibrary|GetMultiIndex (.material _result) true))) (.Strength2 (Class|VoxelBlueprintLibrary|GetMultiIndex (.material _result) true)) (Class|VoxelMaterialCollectionBase|GetIndexMaterial _materialcollection (.Index3 (Class|VoxelBlueprintLibrary|GetMultiIndex (.material _result) true))) (.Strength3 (Class|VoxelBlueprintLibrary|GetMultiIndex (.material _result) true)) (.Wetness (Class|VoxelBlueprintLibrary|GetMultiIndex (.material _result) true)))
    (else
      (return false 0 0.0 0 0.0 0 0.0 0 0.0 0.0))))