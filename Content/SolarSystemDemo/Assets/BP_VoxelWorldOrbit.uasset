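; Solar system demo actor, apparently a voxel world planet, that orbits the world origin and spins on its own axis.
; Each Tick advances an orbit angle to teleport the actor around a circle in the XY plane, and a separate angle to rotate it about UpAxis.
; It lazily finds and caches the first BP_SolarSystemPawn, then updates that pawn's Center to the moving actor's location every frame.
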(event EventTick
  (params (DeltaSeconds :type Float%20%28single-precision%29))
  (bind _output_get (Variables|Default|SetCurrentOrbit (+ (* DeltaSeconds (Variables|Default|GetOrbitSpeed)) (Variables|Default|GetCurrentOrbit))))
  (Transformation|SetActorLocation (* (Math|Vector|MakeVector (Math|Trig|Cos(Radians) _output_get) (Math|Trig|Sin(Radians) _output_get) 0.0) (Variables|Default|GetDistanceToSun)) false true)
  (bind _output_get_2 (Variables|Default|SetCurrentRotation (+ (Variables|Default|GetCurrentRotation) (* (Variables|Default|GetRotateSpeed) DeltaSeconds))))
  (Transformation|SetActorRotation (Math|Vector|RotatorfromAxisandAngle (Variables|Default|GetUpAxis) _output_get_2) true)
  (Utilities|IsValid (Variables|Default|GetPawn)
    (:Is%20Valid
      (Variables|/Game/SolarSystemDemo/Vehicle/BP_SolarSystemPawn.BP_SolarSystemPawn_C|SetCenter (stale _output_get_3) (Transformation|GetActorLocation) :!label _label))
    (:Is%20Not%20Valid
      (bind _outactors (Actor|GetAllActorsOfClass "/Game/SolarSystemDemo/Vehicle/BP_SolarSystemPawn.BP_SolarSystemPawn_C"))
      (if (>= (Utilities|Array|Length _outactors) 1)
        (bind _output_get_3 (Variables|Default|SetPawn (Utilities|Array|Get(acopy) _outactors)))
        (goto _label)))))

(fn ConstructionScript)